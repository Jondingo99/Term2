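; AI controller for Term2 that drives its pawn with the BT_Term2Base behavior tree.
; On BeginPlay it starts the tree and writes the location of the first Term2LevelEndTrigger found to the Destination blackboard key.
; Each tick it copies the game state's IsPlaying flag into the blackboard so the tree can react to play state.
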(event EventBeginPlay
  (Development|PrintString "AI BeginPlay")
  (AI|RunBehaviorTree "/Game/Term2/Blueprints/Characters/BT_Term2Base.BT_Term2Base")
  (bind _outactors (Actor|GetAllActorsOfClass "/Script/Term2.Term2LevelEndTrigger"))
  (if (> (Utilities|Array|Length _outactors) 0)
    (AI|Components|Blackboard|SetValueasVector (Variables|Default|GetBlackboard) (Utilities|Name|MakeLiteralName "Destination") (Transformation|GetActorLocation (Utilities|Array|Get(acopy) _outactors)))))

(event EventTick
  (params (DeltaSeconds :type Float%20%28single-precision%29))
  (bind _asterm_2game_state_base (Utilities|Casting|CastToTerm2GameStateBase (Game|GetGameState)))
  (AI|Components|Blackboard|SetValueasBool (Variables|Default|GetBlackboard) (Utilities|Name|MakeLiteralName "IsPlaying") (Class|Term2GameStateBase|IsPlaying _asterm_2game_state_base)))

(fn ConstructionScript)